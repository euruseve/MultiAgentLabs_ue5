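; AI controller for the avoiding bots that makes them escape from actors they perceive.
; On possession it runs BT_AvoindingBot, then feeds that tree's blackboard from AI Perception updates.
; Each successful sensing prints a debug message and sets EscapeLocation and ShouldEscape.
; The escape point lies a random distance directly away from the sensed actor, projected onto the navmesh.
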(event `self.ReceivePossess`
  (params (PossessedPawn :type "Pawn Object Reference"))
  (`self.RunBehaviorTree` "/Game/_Custom/Lab2/AI/AvoidingBots/BT_AvoindingBot.BT_AvoindingBot"))

(event `self.AIPerception.OnTargetPerceptionUpdated`
  (params (Actor :type "Actor Object Reference") (Stimulus :type "AIStimulus Structure"))
  (bind _returnvalue (`AIBlueprintHelperLibrary.GetBlackboard` null))
  (if (and (!= Actor self) (`.bSuccessfullySensed` (break `AIStimulus` Stimulus)))
    (bind _location (`self.CalcLocation` Actor))
    (`self.PrintSeeing` Actor)
    (`BlackboardComponent.SetValueAsVector` _returnvalue (`self.EscapeLocation  `) _location)
    (`BlackboardComponent.SetValueAsBool` _returnvalue (`self.ShouldEscape`) true)))

(fn `CalcLocation`
  (params (Actor :type "Actor Object Reference"))
  (returns (Location :type "Vector Structure"))
  (bind _returnvalue (`self.K2_GetActorLocation` (`self.K2_GetPawn`)))
  (return (`NavigationSystemV1.K2_ProjectPointToNavigation` (+ (* (`KismetMathLibrary.Normal` (- _returnvalue (`self.K2_GetActorLocation` Actor))) (`KismetMathLibrary.RandomFloatInRange` 450.0 650.0)) _returnvalue))))

(fn `PrintSeeing`
  (params (Actor :type "Actor Object Reference"))
  (`KismetSystemLibrary.PrintString` (`KismetStringLibrary.Concat_StrStr` "Bot \"" (`KismetSystemLibrary.GetDisplayName` self) "\" is seeing \"" (`KismetSystemLibrary.GetDisplayName` Actor) "\"") true true (struct :`R` 0.950661 :`G` 1.0 :`B` 0.138182 :`A` 1.0) 0.7))

(fn `UserConstructionScript`)