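; BP_ActorManager is a manager that shuttles a group of registered agents between two target locations.
; Agents are added to an array through RegisterAgent, and MoveAllTo sends each one a MoveToLocation call with a shared destination.
; A looping timer started on BeginPlay fires RepeatMoving, which uses delays to send all agents to target A, then to target B, in each cycle.
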(event `self.ReceiveBeginPlay`
  (`KismetSystemLibrary.K2_SetTimerDelegate` (delegate `RepeatMoving`) 20.0 true))

(event `MoveAllTo`
  (params (TargetLocation :type "Vector Structure"))
  (for _array_element (`self.Agents`)
    (`/Game/_Custom/Lab3/AI/BP_CentralizedBot.MoveToLocation` _array_element TargetLocation)))

(event `RepeatMoving`
  (`KismetSystemLibrary.Delay` 5.0)
  (`self.MoveAllTo` (`self.K2_GetActorLocation` (`self.TargetLocationA`)))
  (`KismetSystemLibrary.Delay` 5.0)
  (`self.MoveAllTo` (`self.K2_GetActorLocation` (`self.TargetLocationB`))))

(fn `RegisterAgent`
  (params (Agent :type "/Game/_Custom/Lab3/AI/BP_CentralizedBot Object Reference"))
  (`KismetArrayLibrary.Array_Add` (`self.Agents`) Agent))

(fn `UserConstructionScript`)