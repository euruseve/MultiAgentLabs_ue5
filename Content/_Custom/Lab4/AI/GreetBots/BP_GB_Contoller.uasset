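; AI controller for the GreetBot, which runs the BT_GreetBot behavior tree on possession.
; When perception successfully senses another actor, it prints a debug message and sets the ShouldGreet blackboard flag, which it never clears here.
; CalcLocation returns a navmesh-projected point a random distance from the pawn, directly away from a given actor, though nothing in this controller calls it.
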(event `self.ReceivePossess`
  (params (PossessedPawn :type "Pawn Object Reference"))
  (`self.RunBehaviorTree` "/Game/_Custom/Lab4/AI/GreetBots/BT_GreetBot.BT_GreetBot"))

(event `self.AIPerception.OnTargetPerceptionUpdated`
  (params (Actor :type "Actor Object Reference") (Stimulus :type "AIStimulus Structure"))
  (if (and (!= Actor self) (`.bSuccessfullySensed` (break `AIStimulus` Stimulus)))
    (`self.PrintSeeing` Actor)
    (`BlackboardComponent.SetValueAsBool` (`AIBlueprintHelperLibrary.GetBlackboard` null) (`self.ShouldGreet`) true)))

(fn `CalcLocation`
  (params (Actor :type "Actor Object Reference"))
  (returns (Location :type "Vector Structure"))
  (bind _returnvalue (`self.K2_GetActorLocation` (`self.K2_GetPawn`)))
  (return (`NavigationSystemV1.K2_ProjectPointToNavigation` (+ (* (`KismetMathLibrary.Normal` (- _returnvalue (`self.K2_GetActorLocation` Actor))) (`KismetMathLibrary.RandomFloatInRange` 450.0 650.0)) _returnvalue))))

(fn `PrintSeeing`
  (params (Actor :type "Actor Object Reference"))
  (`KismetSystemLibrary.PrintString` (`KismetStringLibrary.Concat_StrStr` "Bot \"" (`KismetSystemLibrary.GetDisplayName` self) "\" is seeing \"" (`KismetSystemLibrary.GetDisplayName` Actor) "\"") true true (struct :`R` 0.950661 :`G` 1.0 :`B` 0.138182 :`A` 1.0) 0.7))

(fn `UserConstructionScript`)